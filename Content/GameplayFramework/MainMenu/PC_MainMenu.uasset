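; Main menu player controller that relays account existence and login checks between the client and the game mode.
; Client events forward requests to Server events, which query GM_MainMenu for account existence, expiry and password validity.
; Results return through Client callbacks to HUD_MainMenu, with an error type for the login check.
; A successful login also stores the user's remaining minutes on the controller.
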(event `Server_CheckIfAccountExist`
  (params (AccountToCheck :type String))
  ;[1 1 1] Check user account
  (bind _asgm_main_menu (cast `/Game/GameplayFramework/MainMenu/GM_MainMenu` (`GameplayStatics.GetGameMode`)))
  (bind _returnvalue (`MainMenuGameMode.CheckAccountExist` _asgm_main_menu AccountToCheck))
  (bind _returnvalue_2 (`MainMenuGameMode.CheckAccountExpired` _asgm_main_menu AccountToCheck))
  (`self.Client_OnAccountChecked` (or _returnvalue_2 _returnvalue)))

(event `Client_AskIfAccountExist`
  (params (AccountToCheck :type String))
  ;[1 1 1] Check user account
  (`self.Server_CheckIfAccountExist` AccountToCheck))

(event `Client_OnAccountChecked`
  (params (Exist :type Boolean))
  ;[1 1 1] Check user account
  (bind _ashud_main_menu (cast `/Game/GameplayFramework/MainMenu/HUD_MainMenu` (`self.GetHUD`)))
  (`/Game/GameplayFramework/MainMenu/HUD_MainMenu.Client_OnAccountChecked` _ashud_main_menu Exist))

(event `Client_CheckPasswordAndAccount`
  (params (Account :type String) (Password :type String))
  ;[1 1 1] Check user password
  (`self.Server_CheckPasswordAndAccount` Account Password))

(event `Server_CheckPasswordAndAccount`
  (params (Account :type String) (Password :type String))
  ;[1 1 1] Check user password
  (bind _asgm_main_menu (cast `/Game/GameplayFramework/MainMenu/GM_MainMenu` (`GameplayStatics.GetGameMode`)))
  (bind _returnvalue (`MainMenuGameMode.CheckAccountExist` _asgm_main_menu Account))
  (if _returnvalue
    (bind _returnvalue_2 (`MainMenuGameMode.CheckUserAccount` _asgm_main_menu Account Password))
    (if _returnvalue_2
      (bind _returnvalue_3 (`MainMenuGameMode.GetUserTimeLeft` _asgm_main_menu Account))
      (`self.Client_OnCheckPasswordAndAccount` false "NewEnumerator0" _returnvalue_3)
      (else
        (`self.Client_OnCheckPasswordAndAccount` true "NewEnumerator1")))
    (else
      (bind _returnvalue_4 (`MainMenuGameMode.CheckAccountExpired` _asgm_main_menu Account))
      (`self.Client_OnCheckPasswordAndAccount` true (select `bool` _returnvalue_4 :`false` "NewEnumerator0" :`true` "NewEnumerator2" :!type "/Game/Misc/E_LoginError Enum")))))

(event `Client_OnCheckPasswordAndAccount`
  (params (Error :type Boolean) (ErrorType :type "/Game/Misc/E_LoginError Enum" :default "NewEnumerator0") (UserTimeLeft :type Integer))
  ;[1 1 1] Check user password
  (bind _ashud_main_menu (cast `/Game/GameplayFramework/MainMenu/HUD_MainMenu` (`self.GetHUD`)))
  (`/Game/GameplayFramework/MainMenu/HUD_MainMenu.Client_OnCheckPasswordAndAccount` _ashud_main_menu Error ErrorType)
  (if (not Error)
    (set `self.User Minutes Left` UserTimeLeft)))

(fn `UserConstructionScript`)