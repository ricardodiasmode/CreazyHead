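; Camera reader actor that supplies webcam, scene capture or player-mode images for OpenCV and shows raw and processed results on two screen components.
; BeginPlay creates the screen materials, opens the selected capture device and enables the chosen input mode.
; Camera media is drawn into a render target on Tick and on each video frame, while player mode draws the processed material to a screen target.
; Validation events reset out-of-range camera and track IDs.
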(event `self.ReceiveBeginPlay`
  (bind _mediaplayer (`self.MediaPlayer`))
  (`parent.ReceiveBeginPlay`)
  (bind _returnvalue (`PrimitiveComponent.CreateDynamicMaterialInstance` (`self.Screen_Post`) 0 "/Game/FaceDetector/M_OpenCVPost.M_OpenCVPost" "None"))
  (set `self.Material_Post` _returnvalue)
  (bind _returnvalue_2 (`PrimitiveComponent.CreateDynamicMaterialInstance` (`self.Screen_Raw`) 0 "/Game/FaceDetector/M_OpenCVPlayer.M_OpenCVPlayer" "None"))
  (set `self.Material_RenderTarget` _returnvalue_2)
  (bind _outdevices (`MediaBlueprintFunctionLibrary.EnumerateVideoCaptureDevices` -1))
  (bind (_output_displayname _output_url) (break `MediaCaptureDevice` (`|GetArrayItem` _outdevices (`self.CameraID`))))
  (`MediaPlayer.OpenUrl` (`self.MediaPlayer`) _output_url)
  (switch `EInputMode` (`self.InputMode`)
    (:`Camera`
      (`self.EnableCameraModeBp`)
      (`KismetSystemLibrary.Delay` 0.2)
      (`MediaPlayer.SelectTrack` _mediaplayer "Video" (`self.VideoTrackID`))
      (`KismetSystemLibrary.Delay` 0.2)
      (`MediaPlayer.Play` _mediaplayer))
    (:`Scene`
      (`self.EnableSceneCapture`))
    (:`Player`
      (`self.EnablePlayerModeBp`)))
  (`KismetSystemLibrary.Delay` 0.2)
  (`MaterialInstanceDynamic.SetTextureParameterValue` (`self.Material_Post`) "OpenCV_Texture" (`self.OpenCV_Texture2D`)))

(event `self.ReceiveTick`
  (params (DeltaSeconds :type "Float (single-precision)"))
  (bind _rendertarget (`self.RenderTarget`))
  (bind _material_cameraraw (`self.Material_CameraRaw`))
  (`parent.ReceiveTick` DeltaSeconds)
  (`/Engine/EditorBlueprintResources/StandardMacros.IsValid` _rendertarget
    (:`Is Valid`
      (`/Engine/EditorBlueprintResources/StandardMacros.IsValid` _material_cameraraw
        (:`Is Valid`
          (`KismetRenderingLibrary.DrawMaterialToRenderTarget` _rendertarget _material_cameraraw))))))

(event `self.OnNextVideoFrame`
  (switch `EInputMode` (`self.InputMode`)
    (:`Camera`
      (`self.RenderCamera`))
    (:`Scene`
      (`/Engine/EditorBlueprintResources/StandardMacros.IsValid` (`self.RenderTarget`)
        (:`Is Valid`
          (`/Engine/EditorBlueprintResources/StandardMacros.IsValid` (`self.Scene_Capture`)))))
    (:`Player`
      (`KismetRenderingLibrary.DrawMaterialToRenderTarget` (`self.RenderTarget_PlayerScreen`) (`self.Material_Post`)))))

(event `self.ValidateCameraID`
  (bind _cameraid (`self.CameraID`))
  (if (< _cameraid 0)
    (set `self.CameraID` 0)
    (else
      (bind _outdevices (`MediaBlueprintFunctionLibrary.EnumerateVideoCaptureDevices` -1))
      (if (>= _cameraid (`KismetArrayLibrary.Array_Length` _outdevices))
        (set `self.CameraID` 0)))))

(event `self.ValidateVideoTrackID`
  (bind _videotrackid (`self.VideoTrackID`))
  (if (< _videotrackid 0)
    (set `self.VideoTrackID` 0)
    (elif (>= _videotrackid (`MediaPlayer.GetNumTracks` (`self.MediaPlayer`) "Audio"))
      (set `self.VideoTrackID` 0))))

(fn `EnableCameraModeBp`
  (`self.DisablePlayerMode`)
  (`self.EnableCameraMode`)
  (bind _outdevices (`MediaBlueprintFunctionLibrary.EnumerateVideoCaptureDevices` -1))
  (`MediaPlayer.OpenUrl` (`self.MediaPlayer`) (`.Url` (break `MediaCaptureDevice` (`|GetArrayItem` _outdevices (`self.CameraID`)))))
  (`/Engine/EditorBlueprintResources/StandardMacros.IsValid` (`self.Material_CameraRaw`)
    (:`Is Not Valid`
      (bind _returnvalue (`PrimitiveComponent.CreateDynamicMaterialInstance` (`self.Screen_Raw`) 0 "/Game/FaceDetector/M_MediaRaw.M_MediaRaw" "None"))
      (set `self.Material_CameraRaw` _returnvalue)
      (`MaterialInstanceDynamic.SetTextureParameterValue` (`self.Material_RenderTarget`) "OpenCV_Texture" (`self.RenderTarget`)))))

(fn `EnablePlayerModeBp`
  (`self.EnablePlayerMode`)
  (`MaterialInstanceDynamic.SetTextureParameterValue` (`self.Material_RenderTarget`) "OpenCV_Texture" (`self.RenderTarget_32Bit`)))

(fn `EnableSceneCapture`
  (`self.DisablePlayerMode`)
  (bind _scene_capture (`self.Scene_Capture`)
    (:`then`
      (bind _rendertarget (`self.RenderTarget`)
        (:`then`
          (`self.Material_RenderTarget`
            (:`then`
              _)
            (:`else`
              (bind _returnvalue (`PrimitiveComponent.CreateDynamicMaterialInstance` (`self.Screen_Raw`) 0 null "None"))
              (set `self.Material_RenderTarget` _returnvalue)))
          (set `SceneCaptureComponent.bCaptureEveryFrame` false _scene_capture)
          (set `SceneCaptureComponent2D.TextureTarget` _rendertarget _scene_capture)
          (`MaterialInstanceDynamic.SetTextureParameterValue` (`self.Material_RenderTarget`) "OpenCV_Texture" (`self.RenderTarget`)))
        (:`else`)))
    (:`else`)))

(fn `RenderCamera`
  (bind _rendertarget (`self.RenderTarget`))
  (bind _material_cameraraw (`self.Material_CameraRaw`))
  (`/Engine/EditorBlueprintResources/StandardMacros.IsValid` _rendertarget
    (:`Is Valid`
      (`/Engine/EditorBlueprintResources/StandardMacros.IsValid` _material_cameraraw
        (:`Is Valid`
          (`KismetRenderingLibrary.DrawMaterialToRenderTarget` _rendertarget _material_cameraraw))))))

(fn `UserConstructionScript`)