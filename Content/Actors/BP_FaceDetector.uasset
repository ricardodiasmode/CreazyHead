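; BP_FaceDetector displays frame textures on the planes of BP_SkmDancer actors and offers brightness controls for them.
; After a short delay at BeginPlay, it gives each dancer's plane a dynamic M_FaceDetector material, having first copied the chroma key setting from GeneralGameInstance.
; Tick pushes each FrameAsTexture entry into the material with the matching index.
; Increase and decrease events step the Brightness parameter on all those materials.
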(event `self.ReceiveBeginPlay`
  (bind _asgeneral_game_instance (cast `/Game/GameplayFramework/GeneralGameInstance` (`GameplayStatics.GetGameInstance`)))
  (set `self.WithChromaKey` (`/Game/GameplayFramework/GeneralGameInstance.UsingChromaKey` _asgeneral_game_instance))
  (`KismetSystemLibrary.Delay` 4.0)
  (bind _outactors (`GameplayStatics.GetAllActorsOfClass` "/Game/Actors/BP_SkmDancer.BP_SkmDancer_C"))
  (for _array_element _outactors
    (bind _plane (`/Game/Actors/BP_SkmDancer.Plane` _array_element))
    (bind _returnvalue (`PrimitiveComponent.CreateDynamicMaterialInstance` _plane 0 "/Game/Materials/M_FaceDetector.M_FaceDetector" "None"))
    (`KismetArrayLibrary.Array_Add` (`self.DynMat`) _returnvalue)
    (`PrimitiveComponent.SetMaterial` _plane 0 _returnvalue)))

(event `self.ReceiveTick`
  (params (DeltaSeconds :type "Float (single-precision)"))
  (bind _dynmat (`self.DynMat`))
  (if (> (`KismetArrayLibrary.Array_Length` _dynmat) 0)
    (for (_array_element _array_index) (`self.FrameAsTexture`)
      (`MaterialInstanceDynamic.SetTextureParameterValue` (`|GetArrayItem` _dynmat _array_index) "Texture" _array_element))))

(event `IncreaseBrightness`
  (for _array_element (`self.DynMat`)
    (bind _returnvalue (`MaterialInstanceDynamic.K2_GetScalarParameterValue` _array_element "Brightness"))
    (`MaterialInstanceDynamic.SetScalarParameterValue` _array_element "Brightness" (+ _returnvalue 0.25))))

(event `DecreaseBrightness`
  (for _array_element (`self.DynMat`)
    (bind _returnvalue (`MaterialInstanceDynamic.K2_GetScalarParameterValue` _array_element "Brightness"))
    (`MaterialInstanceDynamic.SetScalarParameterValue` _array_element "Brightness" (+ _returnvalue -0.25))))

(fn `UserConstructionScript`)